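; BP_Duel_Pawn is a player pawn that handles cursor display, material assignment and session hotkeys in what appears to be a networked duel.
; On BeginPlay it shows the mouse cursor and sets its static mesh material by local control, applying MaterialRemote when locally controlled and MaterialLocal otherwise.
; Space, on a locally controlled pawn, runs a servertravel console command to the Duel_Scripting map, and Escape quits the game.
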(event EventBeginPlay
  (Variables|/Script/Engine.PlayerController|SetbShowMouseCursor (Game|GetPlayerController 0) true)
  (Rendering|Material|SetMaterial (Actor|GetComponentbyClass "/Script/Engine.StaticMeshComponent") 0 (select (Pawn|IsLocallyControlled) (Variables|Default|GetMaterialRemote) (Variables|Default|GetMaterialLocal))))

(event Collision|EventActorBeginOverlap
  (params (OtherActor :type Actor%20Object%20Reference)))

(event EventTick
  (params (DeltaSeconds :type Float%20%28single-precision%29)))

(event Input|KeyboardEvents|SpaceBar
  (params (Key :type Key%20Structure :default "None"))
  (:Pressed
    (if (Pawn|IsLocallyControlled)
      (Development|ExecuteConsoleCommand "servertravel Duel_Scripting" 0))))

(event Input|KeyboardEvents|Escape
  (params (Key :type Key%20Structure :default "None"))
  (:Pressed
    (Game|QuitGame (Game|GetPlayerController 0) "Quit" true)))

(fn ConstructionScript)